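; Chicken character that roams under AIC_Roaming, flees from the first-person player and can be picked up.
; A human detection volume sets IsPlayerNear and switches the AI controller between Run4Life and FreeToGo.
; A chicken detection volume spreads that state on overlap, telling the other chicken's controller to flee or roam.
; Interact returns the mesh and triggers a short-delayed destroy, while the run animation loops from BeginPlay.
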(event OnComponentBeginOverlap(DetectionChicken)
  (params (OverlappedComponent :type Primitive%20Component%20Object%20Reference) (OtherActor :type Actor%20Object%20Reference) (OtherComp :type Primitive%20Component%20Object%20Reference) (OtherBodyIndex :type Integer) (bFromSweep :type Boolean) (SweepResult :type Hit%20Result%20Structure%20%28by%20ref%29))
  ;[1 1 1] Interaction avec les autres poulets
  (bind _asbp_chicken_final (Utilities|Casting|CastToBP_ChickenFinal OtherActor))
  (bind _output_get (Variables|Default|SetLeChickens (Utilities|Array|MakeArray _asbp_chicken_final)))
  (for _array_element _output_get
    (CallFunction|AlertChicken _array_element)))

(event OnComponentBeginOverlap(DetectionHuman)
  (params (OverlappedComponent :type Primitive%20Component%20Object%20Reference) (OtherActor :type Actor%20Object%20Reference) (OtherComp :type Primitive%20Component%20Object%20Reference) (OtherBodyIndex :type Integer) (bFromSweep :type Boolean) (SweepResult :type Hit%20Result%20Structure%20%28by%20ref%29))
  ;[1 1 1] Detection joueur dans les horizons
  (Utilities|Casting|CastToBP_FirstPersonCharacter OtherActor)
  (bind _asaic_roaming (Utilities|Casting|CastToAIC_Roaming (Pawn|GetController)))
  (Default|Run4Life _asaic_roaming)
  (Development|PrintString "Run" true true "(R=1.000000,G=0.127857,B=0.237593,A=1.000000)")
  (Variables|Default|SetIsPlayerNear true))

(event OnComponentEndOverlap(DetectionHuman)
  (params (OverlappedComponent :type Primitive%20Component%20Object%20Reference) (OtherActor :type Actor%20Object%20Reference) (OtherComp :type Primitive%20Component%20Object%20Reference) (OtherBodyIndex :type Integer))
  ;[1 1 1] Detection joueur dans les horizons
  (Utilities|Casting|CastToBP_FirstPersonCharacter OtherActor)
  (bind _asaic_roaming (Utilities|Casting|CastToAIC_Roaming (Pawn|GetController)))
  (Default|FreetoGo _asaic_roaming)
  (Development|PrintString "Free" true true "(R=0.114653,G=1.000000,B=0.000000,A=1.000000)")
  (Variables|Default|SetIsPlayerNear false))

(event Custom|Destroy%20Item
  ;[1 1 1] Quand joueur prend poulet
  (Utilities|FlowControl|Delay 0.2)
  (Actor|DestroyActor))

(event EventBeginPlay
  ;[1 1 1] Animations run
  (Components|Animation|PlayAnimation (Variables|Character|GetMesh) "/Game/Fab/Chicken/run.run" true))

(fn ConstructionScript)

(fn NewFunction
  (params (KeyName :type Name%20%28by%20ref%29) (self2 :type Blackboard%20Component%20Object%20Reference))
  (|CollapseGraph self2 KeyName))

(fn AlertChicken
  (params (PouletsConcernes :type BP%20Chicken%20Final%20Object%20Reference))
  (Development|PrintString "avertissement other chciekn")
  (bind _asaic_roaming (Utilities|Casting|CastToAIC_Roaming (Pawn|GetController PouletsConcernes)))
  (if (Variables|Default|GetIsPlayerNear)
    (Default|Run4Life _asaic_roaming)
    (else
      (Default|FreetoGo _asaic_roaming))))

(fn Interact
  (Development|PrintString "into chicken space")
  (CallFunction|DestroyItem)
  (return (Variables|Character|GetMesh)))